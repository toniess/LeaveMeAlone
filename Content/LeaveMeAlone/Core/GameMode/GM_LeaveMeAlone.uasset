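; GM_LeaveMeAlone is a game mode that runs a match countdown and ends the game when time runs out.
; On BeginPlay it starts a looping one-second timer that decrements GameTime.
; When GameTime reaches zero it pauses the game, shows the WBP_GameOverTimer widget, and switches the player to UI-only input with a visible cursor.
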(event `self.ReceiveBeginPlay`
  (bind _returnvalue (`KismetSystemLibrary.K2_SetTimerDelegate` (delegate `CustomEvent`) 1.0 true))
  (set `self.GameTimerHandle` _returnvalue))

(event `CustomEvent`
  (bind _returnvalue (`GameplayStatics.GetPlayerController` 0))
  (bind _output_get (set `self.GameTime` (- (`self.GameTime`) 1)))
  (if (== _output_get 0)
    (`GameplayStatics.SetGamePaused` true)
    (bind _returnvalue_2 (`|CreateWidget` "/Game/LeaveMeAlone/Core/Widgets/UI/WBP_GameOverTimer.WBP_GameOverTimer_C"))
    (`UserWidget.AddToViewport` _returnvalue_2 0)
    (`WidgetBlueprintLibrary.SetInputMode_UIOnlyEx` _returnvalue _returnvalue_2)
    (set `PlayerController.bShowMouseCursor` true _returnvalue)))

(fn `UserConstructionScript`)