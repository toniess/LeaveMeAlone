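; PC_Player is the player controller that opens the pause and game-over screens.
; Any possessed-pawn change is treated as death: after a short delay it pauses the game and shows WBP_GameOverDeath.
; The Pause input, guarded by OnPause, stops the weapon's auto fire, pauses the game and shows WBP_Pause.
; Both screens switch input to UI-only and show the mouse cursor.
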(event `self.ReceiveBeginPlay`
  (add `self.OnPossessedPawnChanged` (delegate `OnPossessedPawnChanged_Event`)))

(event `OnPossessedPawnChanged_Event` :!signature `self.OnPossessedPawnChanged`
  (params (OldPawn :type "Pawn Object Reference") (NewPawn :type "Pawn Object Reference"))
  (bind _returnvalue (`GameplayStatics.GetPlayerController` 0))
  (`KismetSystemLibrary.Delay` 1.7)
  (`GameplayStatics.SetGamePaused` true)
  (bind _returnvalue_2 (`|CreateWidget` "/Game/LeaveMeAlone/Core/Widgets/UI/WBP_GameOverDeath.WBP_GameOverDeath_C"))
  (bind _output_get (set `self.DeathWidget` _returnvalue_2))
  (`UserWidget.AddToViewport` _output_get 0)
  (`WidgetBlueprintLibrary.SetInputMode_UIOnlyEx` _returnvalue _output_get)
  (set `PlayerController.bShowMouseCursor` true _returnvalue))

(event `InputAction|Pause`
  (params (Key :type "Key Structure"))
  (:`Pressed`
    (if (not (`self.OnPause`))
      (bind _output_get (set `self.WeaponComponent` (`self.GetComponentByClass` (`GameplayStatics.GetPlayerPawn` 0) "/Script/LeaveMeAlone.LMAWeaponComponent")))
      (`LMAWeaponComponent.EndAutoFire` _output_get)
      (set `self.OnPause` true)
      (`GameplayStatics.SetGamePaused` true)
      (bind _returnvalue (`|CreateWidget` "/Game/LeaveMeAlone/Core/Widgets/UI/WBP_Pause.WBP_Pause_C"))
      (bind _output_get_2 (set `self.PauseWidget` _returnvalue))
      (`UserWidget.AddToViewport` _output_get_2 0)
      (`WidgetBlueprintLibrary.SetInputMode_UIOnlyEx` self _output_get_2)
      (set `self.bShowMouseCursor` true))))

(fn `UserConstructionScript`)